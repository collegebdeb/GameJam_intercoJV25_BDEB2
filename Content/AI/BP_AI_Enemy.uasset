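; BP_AI_Enemy is the enemy AI Blueprint that starts the BT_Enemy behavior tree on BeginPlay.
; When PawnSensing sees a pawn and the first player's third-person character is not dead, it flags the sighting and stores that pawn as the blackboard target.
; The death check reads player 0 rather than the seen pawn, and nothing here clears the blackboard values.
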(event OnSeePawn(PawnSensing)
  (params (Pawn :type Pawn%20Object%20Reference))
  (bind _asbp_third_person_character (Utilities|Casting|CastToBP_ThirdPersonCharacter (Game|GetPlayerCharacter 0)))
  (if (not (Variables|/Game/ThirdPerson/Blueprints/BP_ThirdPersonCharacter.BP_ThirdPersonCharacter_C|GetIsDead? _asbp_third_person_character))
    (AI|Components|Blackboard|SetValueasBool (AI|GetBlackboard 0) (Utilities|Name|MakeLiteralName "seeingTarget?") true)
    (AI|Components|Blackboard|SetValueasObject (AI|GetBlackboard 0) (Utilities|Name|MakeLiteralName "targetActor") Pawn)))

(event EventBeginPlay
  (AI|RunBehaviorTree "/Game/AI/BT_Enemy.BT_Enemy"))

(fn ConstructionScript)