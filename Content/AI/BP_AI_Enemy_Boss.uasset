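; AI controller for a boss enemy that shows and hides the boss health bar on screen.
; When PawnSensing sees a Player-tagged pawn and no bar exists, it stores that target and creates the widget, copying Health and MaxHealth from BPC_Stats.
; Each tick, RemoveHealthBar removes the bar when the target is far away and recreates it within a much closer radius, leaving a hysteresis gap.
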(event OnSeePawn(PawnSensing)
  (params (Pawn :type Pawn%20Object%20Reference))
  (bind _self self)
  (bind _returnvalue (Pawn|GetControlledPawn _self))
  (bind _returnvalue_2 (Actor|GetComponentbyClass _returnvalue "/Game/Blueprints/BPC_Stats.BPC_Stats_C"))
  (if (Actor|ActorHasTag Pawn "Player")
    (Variables|Default|GetBossHealthBar
      (:then)
      (:else
        (Variables|Default|SetTargetActor Pawn)
        (bind _returnvalue_3 (UserInterface|CreateWidget "/Game/Widgets/BossHealthBar.BossHealthBar_C"))
        (bind _output_get (Variables|Default|SetBossHealthBar _returnvalue_3))
        (UserInterface|Viewport|AddtoViewport _output_get 0)
        (Variables|/Game/Widgets/BossHealthBar.BossHealthBar_C|SetHealth _output_get (Variables|/Game/Blueprints/BPC_Stats.BPC_Stats_C|Gethealth _returnvalue_2))
        (Variables|/Game/Widgets/BossHealthBar.BossHealthBar_C|SetMax%20Health _output_get (Variables|/Game/Blueprints/BPC_Stats.BPC_Stats_C|GetmaxHealth _returnvalue_2))))))

(event Custom|CreateBarWidget
  (bind _self self)
  (bind _returnvalue (Pawn|GetControlledPawn _self))
  (bind _returnvalue_2 (Actor|GetComponentbyClass _returnvalue "/Game/Blueprints/BPC_Stats.BPC_Stats_C"))
  (bind _returnvalue_3 (UserInterface|CreateWidget "/Game/Widgets/BossHealthBar.BossHealthBar_C"))
  (bind _output_get (Variables|Default|SetBossHealthBar _returnvalue_3))
  (UserInterface|Viewport|AddtoViewport _output_get 0)
  (Variables|/Game/Widgets/BossHealthBar.BossHealthBar_C|SetHealth _output_get (Variables|/Game/Blueprints/BPC_Stats.BPC_Stats_C|Gethealth _returnvalue_2))
  (Variables|/Game/Widgets/BossHealthBar.BossHealthBar_C|SetMax%20Health _output_get (Variables|/Game/Blueprints/BPC_Stats.BPC_Stats_C|GetmaxHealth _returnvalue_2)))

(event EventBeginPlay
  (|CallParentFunction) ; This node is disabled and will not be called.\nDrag off pins to build functionality.
)

(event EventTick
  (params (DeltaSeconds :type Float%20%28single-precision%29))
  (CallFunction|RemoveHealthBar))

(fn ConstructionScript
  (|CallParentFunction))

(fn RemoveHealthBar
  (Variables|Default|GetBossHealthBar
    (:then
      (if (> (Transformation|GetDistanceTo (Variables|Default|GetTargetActor) self) 3e+03)
        (Widget|RemovefromParent (Variables|Default|GetBossHealthBar))
        (Variables|Default|SetBossHealthBar 0)))
    (:else
      (bind _targetactor (Variables|Default|GetTargetActor)
        (:then
          (if (<= (Transformation|GetDistanceTo _targetactor self) 8e+02)
            (CallFunction|CreateBarWidget)))
        (:else)))))