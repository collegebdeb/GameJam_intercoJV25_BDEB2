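; Enemy character that fights with a sword, loses a BPCStats stat with a hit reaction when damaged, and ragdolls on defeat.
; SwordAttack plays the combo montage, while Begin and End trace events start and clear a fast looping timer.
; Each tick of that timer sphere-traces for pawns between two sword points.
; Hitting the tagged player calls its Death outright and stops the current montage.
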(event Custom|Damage%20Trace
  ;[0.15 0.15 0.15 0.5] Sword Traces
  (bind (_outhit _returnvalue) (Collision|SphereTraceForObjects (Transformation|GetWorldLocation (Variables|Default|GetStart%20Sword%20Trace%20Pos)) (Transformation|GetWorldLocation (Variables|Default|GetEnd%20Sword%20Trace%20Pos)) 2e+01 (Utilities|Array|MakeArray "ObjectTypeQuery3") false 0 "ForOneFrame"))
  (if _returnvalue
    (if (Actor|ActorHasTag (.HitActor (Collision|BreakHitResult _outhit)) "Player")
      (bind _asbp_third_person_character (Utilities|Casting|CastToBP_ThirdPersonCharacter (.HitActor (Collision|BreakHitResult _outhit))))
      (Default|Death _asbp_third_person_character "NewEnumerator4")
      (Animation|StopAnimMontage (Animation|GetCurrentMontage :!class /Script/Engine.Character)))))

(event EventBeginSwordTrace
  ;[0.15 0.15 0.15 0.5] Sword Traces
  (bind _returnvalue (Utilities|Time|SetTimerbyEvent (delegate Custom|Damage%20Trace) 0.01 true)))

(event EventEndSwordTrace
  ;[0.15 0.15 0.15 0.5] Sword Traces
  (if (Utilities|Time|IsValidTimerHandle (stale EventBeginSwordTrace _returnvalue))
    (Utilities|Time|ClearandInvalidateTimerbyHandle (stale EventBeginSwordTrace _returnvalue))))

(event Game|Damage|EventAnyDamage
  (params (Damage :type Float%20%28single-precision%29) (DamageType :type Damage%20Type%20Object%20Reference) (InstigatedBy :type Controller%20Object%20Reference) (DamageCauser :type Actor%20Object%20Reference))
  ;[0.06125 0.06125 0.06125] Damage
  (Default|IncreaseValue (Variables|Default|GetBPC_Stats) "NewEnumerator0" (* Damage -1.0))
  (Animation|Montage|PlayMontage (Variables|Character|GetMesh) "/Game/Characters/Animations/Combat_Animations/HitReact_Montage.HitReact_Montage"))

(event EventDefeat
  ;[0.06125 0.06125 0.06125] Defeated
  (Pawn|Components|CharacterMovement|DisableMovement (Variables|Character|GetCharacterMovement))
  (Physics|SetSimulatePhysics (Variables|Character|GetMesh) true))

(fn ConstructionScript)

(fn SwordAttack
  (bind _returnvalue (Animation|PlayAnimMontage "/Game/Characters/Animations/Combat_Animations/AM_AttackCombo.AM_AttackCombo" 1.0 "None"))
  (return _returnvalue))