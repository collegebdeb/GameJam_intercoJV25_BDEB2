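; Boss enemy character Blueprint that takes damage through its stats component and provides a big attack.
; On any damage it subtracts the amount from a stat in BPCStats and starts a hit-react montage.
; It then copies health and max health to the boss health bar on its AI controller, with a bar-creation call on the invalid-controller branch.
; BigAttack plays the attack montage and returns the PlayAnimMontage result.
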(event EventBeginPlay
  (|CallParentFunction))

(event Game|Damage|EventAnyDamage
  (params (Damage :type Float%20%28single-precision%29) (DamageType :type Damage%20Type%20Object%20Reference) (InstigatedBy :type Controller%20Object%20Reference) (DamageCauser :type Actor%20Object%20Reference))
  (bind _bpc_stats (Variables|Default|GetBPC_Stats))
  (Default|IncreaseValue (Variables|Default|GetBPC_Stats) "NewEnumerator0" (* Damage -1.0))
  (Animation|Montage|PlayMontage (Variables|Character|GetMesh) "/Game/Characters/Animations/Combat_Animations/HitReact_Montage.HitReact_Montage"
    (:then
      (bind _asbp_ai_enemy_boss (Utilities|Casting|CastToBP_AI_Enemy_Boss (AI|GetAIController self)))
      (Utilities|IsValid _asbp_ai_enemy_boss
        (:Is%20Valid
          (Variables|/Game/Widgets/BossHealthBar.BossHealthBar_C|SetMax%20Health (Variables|/Game/AI/BP_AI_Enemy_Boss.BP_AI_Enemy_Boss_C|GetBossHealthBar _asbp_ai_enemy_boss) (Variables|/Game/Blueprints/BPC_Stats.BPC_Stats_C|GetmaxHealth _bpc_stats))
          (Variables|/Game/Widgets/BossHealthBar.BossHealthBar_C|SetHealth (Variables|/Game/AI/BP_AI_Enemy_Boss.BP_AI_Enemy_Boss_C|GetBossHealthBar _asbp_ai_enemy_boss) (Variables|/Game/Blueprints/BPC_Stats.BPC_Stats_C|Gethealth _bpc_stats)))
        (:Is%20Not%20Valid
          (Default|CreateBarWidget _asbp_ai_enemy_boss))))))

(fn ConstructionScript
  (|CallParentFunction))

(fn BigAttack
  (bind _returnvalue (Animation|PlayAnimMontage "/Game/Characters/Animations/Combat_Animations/BigAttack_Montage.BigAttack_Montage" 1.0 "None"))
  (return _returnvalue))