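; BP_Bomb is a timed bomb actor that triggers itself five seconds after spawning.
; Trigger enables physics, pops the sphere with an impulse, then shortly after spawns an explosion emitter and hides the bomb visuals.
; A multi-sphere trace finds Player-tagged BP_ThirdPersonCharacters, launches them outward with added lift and calls Death after a brief delay.
; The actor destroys itself a few seconds after exploding, whether or not anything was hit.
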(event Custom|Trigger
  (bind _returnvalue (Transformation|GetActorLocation))
  (bind _spheregeometry (Variables|Default|GetSphereGeometry))
  (Physics|SetSimulatePhysics (Variables|Default|GetSphereGeometry) true)
  (Physics|AddImpulseatLocation _spheregeometry (Math|Vector|MakeVector 0.0 0.0 (.z (Math|Conversions|ToVector(Float) (Variables|Default|GetImpulse)))) (Transformation|GetWorldLocation _spheregeometry) "None")
  (Utilities|FlowControl|Delay 0.3)
  (Effects|SpawnEmitterAttached "/Game/LevelPrototyping/StarterContent/Particles/P_Explosion.P_Explosion" (Variables|Default|GetSphereGeometry) "None" "0, 0, 0" "0, 0, 0" "2.000000,2.000000,2.000000" "SnapToTarget")
  (Rendering|SetVisibility (Variables|Default|GetSphereGeometry) false false)
  (Rendering|SetVisibility (Variables|Default|GetMecheBombe_NS) false false)
  (bind (_outhits _returnvalue_2) (Collision|MultiSphereTraceByChannel _returnvalue _returnvalue 5e+02 "TraceTypeQuery1" false 0 "None"))
  (if _returnvalue_2
    (Utilities|FlowControl|Sequence
      (:then_0
        (Utilities|FlowControl|Delay 3.0 :!label _label)
        (Actor|DestroyActor))
      (:then_1
        (for _array_element _outhits
          (if (Actor|ActorHasTag (.HitActor (Collision|BreakHitResult _array_element)) "Player")
            (bind _asbp_third_person_character (Utilities|Casting|CastToBP_ThirdPersonCharacter (.HitActor (Collision|BreakHitResult _array_element))))
            (Character|LaunchCharacter _asbp_third_person_character (+ (* (Math|Vector|GetForwardVector (Math|Rotator|FindLookatRotation (Transformation|GetActorLocation) (Transformation|GetActorLocation _asbp_third_person_character))) (Variables|Default|GetBombForce)) "0.000000,0.000000,300.000000") false false)
            (Utilities|FlowControl|Delay 0.2)
            (Default|Death _asbp_third_person_character "NewEnumerator7")))))
    (else
      (goto _label))))

(event EventBeginPlay
  (Utilities|FlowControl|Delay 5.0)
  (CallFunction|Trigger))

(event EventTick
  (params (DeltaSeconds :type Float%20%28single-precision%29)))

(fn ConstructionScript)