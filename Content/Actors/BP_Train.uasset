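; Train hazard actor that repeatedly travels a fixed distance in a straight line and kills the player on contact.
; A self-calling event with a short Delay steps it along its negative right vector by CarSpeed without sweep, so its speed depends on frame rate.
; Beyond MaxCarDistance it teleports back to its starting location and restarts.
; The CollisionDamage overlap calls Death on a Player-tagged BP_ThirdPersonCharacter.
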(event OnComponentBeginOverlap(CollisionDamage)
  (params (OverlappedComponent :type Primitive%20Component%20Object%20Reference) (OtherActor :type Actor%20Object%20Reference) (OtherComp :type Primitive%20Component%20Object%20Reference) (OtherBodyIndex :type Integer) (bFromSweep :type Boolean) (SweepResult :type Hit%20Result%20Structure%20%28by%20ref%29))
  (if (Actor|ActorHasTag OtherActor "Player")
    (bind _asbp_third_person_character (Utilities|Casting|CastToBP_ThirdPersonCharacter OtherActor))
    (Default|Death _asbp_third_person_character "NewEnumerator12")))

(event Custom|MoveForward
  (Transformation|SetActorLocation (+ (Transformation|GetActorLocation) (* (* (Transformation|GetActorRightVector) -1.0) (Variables|Default|GetCarSpeed))) false false)
  (Utilities|FlowControl|Delay 0.01)
  (if (> (Math|Vector|Distance(Vector) (Variables|Default|GetInitialLocation) (Transformation|GetActorLocation)) (Variables|Default|GetMaxCarDistance))
    (CallFunction|TeleportBack)
    (else
      (CallFunction|MoveForward))))

(event Custom|TeleportBack
  (Transformation|SetActorLocation (Variables|Default|GetInitialLocation) false false)
  (CallFunction|MoveForward))

(event EventBeginPlay
  (Variables|Default|SetInitialLocation (Transformation|GetActorLocation))
  (CallFunction|MoveForward))

(fn ConstructionScript)