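; BombTrigger_BP is a trigger actor that sets off the nearest BP_Bomb when anything begins overlapping its Box.
; On overlap it scans all BP_Bomb actors, keeps the one closest to itself, and calls Trigger on it if valid.
; ClosestBomb holds the best distance and is never reset, so its starting value limits range and each later search inherits the previous minimum.
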(event OnComponentBeginOverlap(Box)
  (params (OverlappedComponent :type Primitive%20Component%20Object%20Reference) (OtherActor :type Actor%20Object%20Reference) (OtherComp :type Primitive%20Component%20Object%20Reference) (OtherBodyIndex :type Integer) (bFromSweep :type Boolean) (SweepResult :type Hit%20Result%20Structure%20%28by%20ref%29))
  (Variables|Default|SetBombToExplode 0)
  (bind _outactors (Actor|GetAllActorsOfClass "/Game/Actors/BP_Bomb.BP_Bomb_C"))
  (for _array_element _outactors
    (if (<= (Math|Vector|Distance(Vector) (Transformation|GetActorLocation _array_element) (Transformation|GetActorLocation)) (Variables|Default|GetClosestBomb))
      (Variables|Default|SetClosestBomb (Math|Vector|Distance(Vector) (Transformation|GetActorLocation _array_element) (Transformation|GetActorLocation)))
      (Variables|Default|SetBombToExplode _array_element)))
  (bind _bombtoexplode (Variables|Default|GetBombToExplode)
    (:then
      (Default|Trigger _bombtoexplode))
    (:else)))

(event EventBeginPlay)

(event Collision|EventActorBeginOverlap
  (params (OtherActor :type Actor%20Object%20Reference)))

(event EventTick
  (params (DeltaSeconds :type Float%20%28single-precision%29)))

(fn ConstructionScript)