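; Car actor that drives in a straight line along its forward vector and loops back to where it started.
; BeginPlay stores the initial location and starts MoveForward, a self-calling event that uses a short Delay instead of Tick to step by CarSpeed, without sweep.
; Once the car exceeds MaxCarDistance from that location, TeleportBack resets its position and restarts the movement.
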(event Custom|MoveForward
  (Transformation|SetActorLocation (+ (Transformation|GetActorLocation) (* (Transformation|GetActorForwardVector) (Variables|Default|GetCarSpeed))) false false)
  (Utilities|FlowControl|Delay 0.01)
  (if (> (Math|Vector|Distance(Vector) (Variables|Default|GetInitialLocation) (Transformation|GetActorLocation)) (Variables|Default|GetMaxCarDistance))
    (CallFunction|TeleportBack)
    (else
      (CallFunction|MoveForward))))

(event Custom|TeleportBack
  (Transformation|SetActorLocation (Variables|Default|GetInitialLocation) false false)
  (CallFunction|MoveForward))

(event EventBeginPlay
  (Variables|Default|SetInitialLocation (Transformation|GetActorLocation))
  (CallFunction|MoveForward))

(fn ConstructionScript)