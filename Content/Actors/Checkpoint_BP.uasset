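; Checkpoint actor that puts the third-person player character back at its position when its Respawn event is called.
; On BeginPlay it casts player character 0 to BP_ThirdPersonCharacter and caches it.
; Respawn teleports that character slightly above the Arrow component, taking roll and yaw from the arrow and keeping the character's own pitch.
; The graph contains no trigger or activation logic of its own.
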(event Custom|Respawn
  (bind _player (Variables|Default|GetPlayer))
  (bind _arrow (Variables|Default|GetArrow))
  (bind _returnvalue (Transformation|GetWorldRotation _arrow))
  (Transformation|SetActorLocationAndRotation _player (+ (Transformation|GetWorldLocation (Variables|Default|GetArrow)) "0.000000,0.000000,30.000000") (Math|Rotator|MakeRotator (.roll _returnvalue) (.pitch (Transformation|GetActorRotation _player)) (.yaw _returnvalue))))

(event EventBeginPlay
  (bind _asbp_third_person_character (Utilities|Casting|CastToBP_ThirdPersonCharacter (Game|GetPlayerCharacter 0)))
  (Variables|Default|SetPlayer _asbp_third_person_character))

(fn ConstructionScript)