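; Climbing component that lets the player attach to and detach from surfaces in front of them, using a Player reference passed through InitComponent.
; StartClimb runs a short, low forward line trace, then switches movement to slowed Flying and turns the player to face the hit surface.
; Losing the surface while climbing triggers EndClimb, which restores Falling movement and briefly blocks climbing through a delayed CanClimb reset.
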(event Custom|StartClimb
  (bind _player (Variables|Default|GetPlayer))
  (bind _player_2 (Variables|Default|GetPlayer))
  (bind _returnvalue (Transformation|GetActorRotation _player))
  (bind _charactermovement (Variables|/Script/Engine.Character|GetCharacterMovement _player_2))
  (if (Variables|/Game/ThirdPerson/Blueprints/BP_ThirdPersonCharacter.BP_ThirdPersonCharacter_C|GetCanClimb? (Variables|Default|GetPlayer))
    (bind (_outhit _hitfound_) (CallFunction|CheckClimbing))
    (if _hitfound_
      (if (.bBlockingHit (Collision|BreakHitResult _outhit))
        (Variables|/Game/ThirdPerson/Blueprints/BP_ThirdPersonCharacter.BP_ThirdPersonCharacter_C|SetIsClimbing? _player_2 true)
        (Variables|/Script/Engine.CharacterMovementComponent|SetbOrientRotationToMovement _charactermovement false)
        (Pawn|Components|CharacterMovement|SetMovementMode _charactermovement "MOVE_Flying" 0)
        (Variables|/Script/Engine.CharacterMovementComponent|SetMaxFlySpeed _charactermovement 2e+02)
        (Transformation|SetActorRotation _player_2 (Math|Rotator|MakeRotator (.roll _returnvalue) (.pitch _returnvalue) (+ (.yaw (Math|Rotator|MakeRotfromX (.Normal (Collision|BreakHitResult _outhit)))) 1.8e+02)))
        (else
          (CallFunction|EndClimb :!label _label)))
      (elif (Variables|/Game/ThirdPerson/Blueprints/BP_ThirdPersonCharacter.BP_ThirdPersonCharacter_C|GetIsClimbing? (Variables|Default|GetPlayer))
        (goto _label)))))

(event Custom|EndClimb
  (bind _player (Variables|Default|GetPlayer))
  (bind _charactermovement (Variables|/Script/Engine.Character|GetCharacterMovement _player))
  (Utilities|FlowControl|Sequence
    (:then_0
      (Variables|/Game/ThirdPerson/Blueprints/BP_ThirdPersonCharacter.BP_ThirdPersonCharacter_C|SetIsClimbing? _player false)
      (Variables|/Script/Engine.CharacterMovementComponent|SetbOrientRotationToMovement _charactermovement true)
      (Pawn|Components|CharacterMovement|SetMovementMode _charactermovement "MOVE_Falling" 0)
      (Variables|/Script/Engine.CharacterMovementComponent|SetMaxFlySpeed _charactermovement 6e+02))
    (:then_1
      (Variables|/Game/ThirdPerson/Blueprints/BP_ThirdPersonCharacter.BP_ThirdPersonCharacter_C|SetCanClimb? _player false)
      (Utilities|FlowControl|Delay 0.5)
      (Variables|/Game/ThirdPerson/Blueprints/BP_ThirdPersonCharacter.BP_ThirdPersonCharacter_C|SetCanClimb? _player true))))

(event EventBeginPlay)

(fn CheckClimbing
  (bind _player (Variables|Default|GetPlayer))
  (bind _returnvalue (Transformation|GetActorLocation _player))
  (bind _returnvalue_2 (- _returnvalue "0.000000,0.000000,75.000000"))
  (bind (_outhit _returnvalue_3) (Collision|LineTraceByChannel _returnvalue_2 (+ _returnvalue_2 (* (Transformation|GetActorForwardVector _player) 1e+02)) "TraceTypeQuery1" false (Utilities|Array|MakeArray (Variables|Default|GetPlayer)) (Variables|Default|GetDebug)))
  (return _outhit _returnvalue_3))

(fn InitComponent
  (params (Player :type BP%20Third%20Person%20Character%20Object%20Reference))
  (Variables|Default|SetPlayer Player))