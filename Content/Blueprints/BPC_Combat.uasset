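; Player combat component for BP_ThirdPersonCharacter, handling sword combo attacks, directional dodges and damage to Boss-tagged pawns.
; Attack input plays a combo montage, which montage notifies stop unless another press queued the next hit.
; Dodge picks a montage from the player's direction key when controller desired rotation is on, otherwise forward.
; Begin/EndDamageTrace toggle a looping timer that sphere-traces along the sword, with a DoOnce cooldown limiting repeated damage.
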(event Custom|Begin%20Damage%20Trace
  ;[0.15 0.15 0.15 0.5] Sword Traces
  (bind _returnvalue (Utilities|Time|SetTimerbyEvent (delegate Custom|Damage%20Trace) 0.01 true)))

(event Custom|Damage%20Trace
  (bind _player_bp (Variables|Default|GetPlayer%20BP))
  ;[0.15 0.15 0.15 0.5] Sword Traces
  (bind (_outhit _returnvalue) (Collision|SphereTraceForObjects (Transformation|GetWorldLocation (Variables|/Game/ThirdPerson/Blueprints/BP_ThirdPersonCharacter.BP_ThirdPersonCharacter_C|GetStart%20Sword%20Trace%20Pos _player_bp)) (Transformation|GetWorldLocation (Variables|/Game/ThirdPerson/Blueprints/BP_ThirdPersonCharacter.BP_ThirdPersonCharacter_C|GetEnd%20Sword%20Trace%20Pos _player_bp)) 2e+01 (Utilities|Array|MakeArray "ObjectTypeQuery3") false 0 "ForOneFrame"))
  (if _returnvalue
    (if (Actor|ActorHasTag (.HitActor (Collision|BreakHitResult _outhit)) "Boss")
      (Utilities|FlowControl|DoOnce false :!label _label
        (:Completed
          (Game|Damage|ApplyDamage (.HitActor (Collision|BreakHitResult _outhit)) (Variables|Default|GetswordDamage) 0 0)
          (Utilities|FlowControl|Delay 0.3)
          (goto _label Reset))))))

(event Custom|End%20Damage%20Trace
  ;[0.15 0.15 0.15 0.5] Sword Traces
  (if (Utilities|Time|IsValidTimerHandle (stale Custom|Begin%20Damage%20Trace _returnvalue))
    (Utilities|Time|ClearandInvalidateTimerbyHandle (stale Custom|Begin%20Damage%20Trace _returnvalue))))

(event Input|EnhancedActionEvents|EnhancedInputActionIA_Attack
  (params (ActionValue :type Boolean) (ElapsedSeconds :type Float%20%28double-precision%29) (TriggeredSeconds :type Float%20%28double-precision%29) (InputAction :type Input%20Action%20Object%20Reference :default "/Game/ThirdPerson/Input/Actions/IA_Attack.IA_Attack"))
  (bind _player_bp (Variables|Default|GetPlayer%20BP))
  (bind _mesh (Variables|/Script/Engine.Character|GetMesh _player_bp))
  (bind _returnvalue (Components|SkeletalMesh|GetAnimInstance _mesh))
  ;[0.15 0.15 0.15 0.5] Déclenche l'animation d'attaque
  (:Started
    (if (not (Variables|Default|GetisAttacking))
      (Variables|Default|SetisAttacking true)
      (Animation|Montage|PlayMontage (Variables|/Script/Engine.Character|GetMesh (Variables|Default|GetPlayer%20BP)) "/Game/Characters/OldMan/Animations/Combat/OldMan_AM_AttackCombo.OldMan_AM_AttackCombo"
        (:OnCompleted
          (Variables|Default|SetisAttacking false :!label _label)
          (Variables|Default|SetattackCombo false))
        (:OnInterrupted
          (goto _label))
        (:OnNotifyBegin
          ;[0.15 0.15 0.15 0.5] Permet d'arrêter l'animation d'attaque
          (if (and (Variables|Default|GetisAttacking) (Variables|Default|GetattackCombo))
            (Variables|Default|SetattackCombo false)
            (else
              (Animation|Montage|MontageStop _returnvalue 0.2 (Animation|Montage|GetCurrentActiveMontage _returnvalue))
              (Variables|Default|SetisAttacking false)
              (Variables|Default|SetattackCombo false)))))
      (else
        (Variables|Default|SetattackCombo true)))))

(event Input|EnhancedActionEvents|EnhancedInputActionIA_Dodge
  (params (ActionValue :type Boolean) (ElapsedSeconds :type Float%20%28double-precision%29) (TriggeredSeconds :type Float%20%28double-precision%29) (InputAction :type Input%20Action%20Object%20Reference :default "/Game/ThirdPerson/Input/Actions/IA_Dodge.IA_Dodge"))
  (:Started
    (if (not (Variables|Default|GetisDodging?))
      (Variables|Default|SetisDodging? true)
      (Utilities|FlowControl|Sequence
        (:then_0
          (if (Variables|/Script/Engine.CharacterMovementComponent|GetbUseControllerDesiredRotation (Variables|/Script/Engine.Character|GetCharacterMovement (Variables|Default|GetPlayer%20BP)))
            (switch string (Utilities|String|ToString(Text) (Class|KismetInputLibrary|KeyGetDisplayName (Variables|/Game/ThirdPerson/Blueprints/BP_ThirdPersonCharacter.BP_ThirdPersonCharacter_C|GetDirection%20Key (Variables|Default|GetPlayer%20BP)) true))
              (:W
                (Variables|Default|SetmovementDirection "NewEnumerator0"))
              (:A
                (Variables|Default|SetmovementDirection "NewEnumerator1"))
              (:S
                (Variables|Default|SetmovementDirection "NewEnumerator2"))
              (:D
                (Variables|Default|SetmovementDirection "NewEnumerator3")))
            (else
              (Variables|Default|SetmovementDirection "NewEnumerator0"))))
        (:then_1
          (Animation|Montage|PlayMontage (Variables|/Script/Engine.Character|GetMesh (Variables|Default|GetPlayer%20BP)) (Utilities|Select :Index (Variables|Default|GetmovementDirection) :NewEnumerator0 "/Game/Characters/OldMan/Animations/Combat/OldMan_Dodge_F_Montage.OldMan_Dodge_F_Montage" :NewEnumerator1 "/Game/Characters/OldMan/Animations/Combat/OldMan_Dodge_L_Montage.OldMan_Dodge_L_Montage" :NewEnumerator2 "/Game/Characters/OldMan/Animations/Combat/OldMan_Dodge_B_Montage.OldMan_Dodge_B_Montage" :NewEnumerator3 "/Game/Characters/Animations/Combat_Animations/Dodge/Dodge_R_Montage.Dodge_R_Montage")
            (:OnCompleted
              _)
            (:OnInterrupted
              _))
          (Variables|Default|SetisDodging? false))))))

(event EventBeginPlay
  ;[0.15 0.15 0.15 0.5] Récupère le joueur dans le BP
  (bind _asbp_third_person_character (Utilities|Casting|CastToBP_ThirdPersonCharacter (Components|GetOwner)))
  (Variables|Default|SetPlayer%20BP _asbp_third_person_character))