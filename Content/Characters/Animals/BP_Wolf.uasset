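; Wolf enemy that roams random reachable points, chases the player on sight and kills them with a melee attack.
; PawnSensing raises its speed and starts an AI move; on arrival a random montage's notify runs a forward sphere trace that calls the player's Death with a checkpoint index.
; After a kill it loops following the player.
; Sighting also triggers following for non-player pawns, or roaming if the player is already dead.
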(event OnSeePawn(PawnSensing)
  (params (Pawn :type Pawn%20Object%20Reference))
  (bind _returnvalue (Transformation|GetActorLocation))
  (if (and (Actor|ActorHasTag Pawn "Player") (not (Variables|Default|GetKilledPlayer?)))
    (if (not (Variables|/Game/ThirdPerson/Blueprints/BP_ThirdPersonCharacter.BP_ThirdPersonCharacter_C|GetIsDead? (Variables|Default|GetPlayer)))
      (Variables|/Script/Engine.CharacterMovementComponent|SetMaxWalkSpeed (Variables|Character|GetCharacterMovement) 5e+02)
      (AI|AIMoveTo self "0, 0, 0" (Game|GetPlayerCharacter 0) (Variables|Default|GetStoppingDistanceFromPlayer) false
        (:OnSuccess
          (if (not (Variables|Default|GetIsAttacking))
            (Variables|Default|SetIsAttacking true)
            (Animation|Montage|PlayMontage (Variables|Character|GetMesh) (.OutItem (Utilities|Array|Random (Variables|Default|GetAttackMontages)))
              (:OnCompleted
                (Variables|Default|SetIsAttacking false))
              (:OnNotifyBegin
                (bind (_outhits _returnvalue_2) (Collision|MultiSphereTraceForObjects _returnvalue (+ _returnvalue (* (Math|Vector|GetForwardVector (Transformation|GetActorRotation)) (Variables|Default|GetAttackDistance))) 75.0 (Utilities|Array|MakeArray "ObjectTypeQuery3") false (Utilities|Array|MakeArray self) "None"))
                (if _returnvalue_2
                  (bind _array_element (Utilities|Array|ForEachLoopwithBreak _outhits :!label _label)
                    (:LoopBody
                      (if (Actor|ActorHasTag (.HitActor (Collision|BreakHitResult _array_element)) "Player")
                        (Default|Death (Variables|Default|GetPlayer) "NewEnumerator8" (Variables|Default|GetDeath%20Checkpoint%20Index))
                        (Variables|Default|SetKilledPlayer? true)
                        (Variables|/Script/Engine.CharacterMovementComponent|SetMaxWalkSpeed (Variables|Character|GetCharacterMovement) 4e+02)
                        (CallFunction|FollowPlayer)
                        (goto _label Break))))))))))
      (else
        (CallFunction|MoveAround)))
    (else
      (CallFunction|FollowPlayer))))

(event Custom|MoveAround
  (if (not (Variables|Default|GetKilledPlayer?))
    (Variables|/Script/Engine.CharacterMovementComponent|SetMaxWalkSpeed (Variables|Character|GetCharacterMovement) 2.5e+02)
    (if true
      (AI|AIMoveTo self (.RandomLocation (AI|Navigation|GetRandomReachablePointinRadius (Transformation|GetActorLocation) 5e+03 0 0)) 0 5.0 false
        (:OnSuccess
          (Utilities|FlowControl|Delay 3.0)
          (CallFunction|MoveAround))))))

(event Custom|FollowPlayer
  (AI|AIMoveTo self "0, 0, 0" (Game|GetPlayerCharacter 0) 5e+02 false
    (:OnSuccess
      (Utilities|FlowControl|Delay 1.0)
      (CallFunction|FollowPlayer))
    (:OnFail
      (CallFunction|FollowPlayer))))

(event EventBeginPlay
  (bind _asbp_third_person_character (Utilities|Casting|CastToBP_ThirdPersonCharacter (Game|GetPlayerCharacter 0)))
  (Variables|Default|SetPlayer _asbp_third_person_character)
  (CallFunction|MoveAround))

(event Collision|EventActorBeginOverlap
  (params (OtherActor :type Actor%20Object%20Reference)))

(fn ConstructionScript)